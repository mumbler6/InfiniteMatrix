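; BP_Enemy is a short-lived enemy actor that expires 3.5 seconds after spawning and reacts to overlaps on its sphere component.
; A BP_Bullet overlap destroys it and adds score to BP_Player.
; A BP_Player overlap destroys it and subtracts health, flagging death and showing the restart display at zero or below.
; Both hits play a world camera shake at the player's location, with all player state written directly through casts.
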(event `self.ReceiveBeginPlay`
  (`self.SetLifeSpan` 3.5))

(event `self.Sphere1.OnComponentBeginOverlap`
  (params (OverlappedComponent :type "PrimitiveComponent Object Reference") (OtherActor :type "Actor Object Reference") (OtherComp :type "PrimitiveComponent Object Reference") (OtherBodyIndex :type Integer) (bFromSweep :type Boolean) (SweepResult :type "HitResult Structure (by ref)"))
  (cast `/Game/InfiniteMatrix/Blueprints/BP_Bullet` OtherActor
    (:`then`
      (`self.K2_DestroyActor`)
      (bind _asbp_player (cast `/Game/InfiniteMatrix/Blueprints/BP_Player` (`GameplayStatics.GetPlayerPawn` 0)))
      (set `/Game/InfiniteMatrix/Blueprints/BP_Player.Score` (+ (`/Game/InfiniteMatrix/Blueprints/BP_Player.Score` _asbp_player) 250) _asbp_player)
      (`GameplayStatics.PlayWorldCameraShake` "/Game/InfiniteMatrix/Blueprints/BP_CamerShake.BP_CamerShake_C" (`self.K2_GetActorLocation` _asbp_player) 0.0 500.0))
    (:`CastFailed`
      (bind _asbp_player_2 (cast `/Game/InfiniteMatrix/Blueprints/BP_Player` OtherActor))
      (`self.K2_DestroyActor`)
      (bind _output_get (set `/Game/InfiniteMatrix/Blueprints/BP_Player.Health` (- (`/Game/InfiniteMatrix/Blueprints/BP_Player.Health` _asbp_player_2) 20.0) _asbp_player_2))
      (if (<= _output_get 0.0)
        (set `/Game/InfiniteMatrix/Blueprints/BP_Player.IsDead` true _asbp_player_2)
        (`/Game/InfiniteMatrix/Blueprints/BP_Player.DisplayRestart` _asbp_player_2))
      (`GameplayStatics.PlayWorldCameraShake` "/Game/InfiniteMatrix/Blueprints/BP_CamerShake.BP_CamerShake_C" (`self.K2_GetActorLocation` _asbp_player_2) 0.0 500.0))))

(fn `UserConstructionScript`)