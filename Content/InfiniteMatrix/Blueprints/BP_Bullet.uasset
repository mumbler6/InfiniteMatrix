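; BP_Bullet is a short-lived projectile in InfiniteMatrix that destroys itself one second after spawning.
; Each tick it moves along world X without sweeping, at its forward speed plus a bonus that scales with the player's score.
; Its Box overlap destroys the bullet on contact with any mesh component or a BP_Enemy, and applies no damage itself.
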(event `self.ReceiveBeginPlay`
  (`self.SetLifeSpan` 1.0))

(event `self.ReceiveTick`
  (params (DeltaSeconds :type "Float (single-precision)"))
  (`self.K2_AddActorWorldOffset` (`KismetMathLibrary.MakeVector` (* DeltaSeconds (+ (`self.ForwardSpeed`) (/ (`/Game/InfiniteMatrix/Blueprints/BP_Player.Score` (`self.Player`)) 7))))))

(event `self.Box.OnComponentBeginOverlap`
  (params (OverlappedComponent :type "PrimitiveComponent Object Reference") (OtherActor :type "Actor Object Reference") (OtherComp :type "PrimitiveComponent Object Reference") (OtherBodyIndex :type Integer) (bFromSweep :type Boolean) (SweepResult :type "HitResult Structure (by ref)"))
  (cast `MeshComponent` OtherComp
    (:`then`
      _)
    (:`CastFailed`
      (cast `/Game/InfiniteMatrix/Blueprints/BP_Enemy` OtherActor)))
  (`self.K2_DestroyActor`))

(fn `UserConstructionScript`)